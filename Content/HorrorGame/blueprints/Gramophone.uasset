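; Gramophone is an interactable horror-game prop that starts or stops its GramophoneList audio when E is pressed nearby.
; A Box overlap enables input for player controller 0 and end overlap disables it, without checking which actor overlaps.
; Each press flips the IsPlayable flag to either play from the beginning or stop.
; The skeletal mesh rotation on play adds zero, so it has no visible effect.
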(event `self.Box.OnComponentBeginOverlap`
  (params (OverlappedComponent :type "PrimitiveComponent Object Reference") (OtherActor :type "Actor Object Reference") (OtherComp :type "PrimitiveComponent Object Reference") (OtherBodyIndex :type Integer) (bFromSweep :type Boolean) (SweepResult :type "HitResult Structure (by ref)"))
  (`self.EnableInput` (`GameplayStatics.GetPlayerController` 0)))

(event `Key|E`
  (params (Key :type "Key Structure" :default "AnyKey"))
  (:`Pressed`
    (if (`self.IsPlayable`)
      (set `self.IsPlayable` false)
      (`SceneComponent.K2_AddLocalRotation` :`self` (`self.SkeletalMesh`))
      (`AudioComponent.Play` (`self.GramophoneList`) 0.0)
      (else
        (set `self.IsPlayable` true)
        (`AudioComponent.Stop` (`self.GramophoneList`))))))

(event `self.Box.OnComponentEndOverlap`
  (params (OverlappedComponent :type "PrimitiveComponent Object Reference") (OtherActor :type "Actor Object Reference") (OtherComp :type "PrimitiveComponent Object Reference") (OtherBodyIndex :type Integer))
  (`self.DisableInput` (`GameplayStatics.GetPlayerController` 0)))

(fn `UserConstructionScript`)