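; DoorWay is an interactable door Blueprint that the player swings open and shut with E while inside its Box trigger.
; Box overlap begin and end enable and disable input for player controller 0, without checking which actor overlaps.
; DoorStatus toggles the DoorRotation timeline between play and reverse, driving the Door's relative yaw.
; Playing triggers an attenuated wood movement sound, while reversing triggers a stop sound after a short delay.
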(event `self.Box.OnComponentBeginOverlap`
  (params (OverlappedComponent :type "PrimitiveComponent Object Reference") (OtherActor :type "Actor Object Reference") (OtherComp :type "PrimitiveComponent Object Reference") (OtherBodyIndex :type Integer) (bFromSweep :type Boolean) (SweepResult :type "HitResult Structure (by ref)"))
  (`self.EnableInput` (`GameplayStatics.GetPlayerController` 0)))

(event `Key|E`
  (params (Key :type "Key Structure" :default "AnyKey"))
  (:`Pressed`
    (if (`self.DoorStatus`)
      (set `self.DoorStatus` false)
      (`GameplayStatics.PlaySoundAtLocation` "/Game/HorrorGame/Audio/door1_move.door1_move" (`SceneComponent.K2_GetComponentLocation` (`self.wood_move1`)) (struct) 1.0 1.0 0.0 "/Game/HorrorGame/blueprints/GramophoneAttenuation.GramophoneAttenuation")
      (bind (_direction _doorrot) (`Timeline|DoorRotation` :!label _label)
        (:`Update`
          (`SceneComponent.K2_SetRelativeRotation` (`self.Door`) (`KismetMathLibrary.MakeRotator` 0.0 0.0 _doorrot) false false)))
      (else
        (`|ExecutionSequence`
          (:`then_0`
            (set `self.DoorStatus` true)
            (goto _label :!via `Reverse`))
          (:`then_1`
            (`KismetSystemLibrary.Delay` 1.0)
            (`GameplayStatics.PlaySoundAtLocation` "/Game/HorrorGame/Audio/wood_stop1.wood_stop1" (`SceneComponent.K2_GetComponentLocation` (`self.wood_move1`)) (struct) 1.0 1.0 0.0 "/Game/HorrorGame/blueprints/GramophoneAttenuation.GramophoneAttenuation")))))))

(event `self.Box.OnComponentEndOverlap`
  (params (OverlappedComponent :type "PrimitiveComponent Object Reference") (OtherActor :type "Actor Object Reference") (OtherComp :type "PrimitiveComponent Object Reference") (OtherBodyIndex :type Integer))
  (`self.DisableInput` (`GameplayStatics.GetPlayerController` 0)))

(fn `UserConstructionScript`)