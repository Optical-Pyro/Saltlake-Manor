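; Thunder actor that produces timed lightning flashes with thunder audio for the horror game.
; Tick starts a latent chain that waits, plays the Thunder component, then briefly spikes a PointLight to extreme intensity.
; The light drops to zero after a random delay between MinTime and MaxTime, and the latent delays pace the repeats instead of a timer.
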(event `self.ReceiveTick`
  (params (DeltaSeconds :type "Float (single-precision)"))
  (bind _pointlight (`self.PointLight`))
  (`KismetSystemLibrary.Delay` 10.0)
  (`AudioComponent.Play` (`self.Thunder`) 0.0)
  (`KismetSystemLibrary.Delay` 0.2)
  (`LightComponent.SetIntensity` _pointlight 10000000.0)
  (`KismetSystemLibrary.Delay` (`KismetMathLibrary.RandomFloatInRange` (`self.MinTime`) (`self.MaxTime`)))
  (`LightComponent.SetIntensity` _pointlight 0.0))

(fn `UserConstructionScript`)