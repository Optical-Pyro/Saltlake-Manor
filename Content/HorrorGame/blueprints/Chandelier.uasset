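; Chandelier Blueprint for the horror game that switches eight point lights on and off together.
; The LightOn and LightOff events each feed a separate input of a shared Chandelier sub-graph.
; That sub-graph sets the intensity of all the lights at once, to a fixed bright level or to zero.
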(event `Light On`
  (`LightComponent.SetIntensity` (`self.PointLight`) 2500.0)
  (`LightComponent.SetIntensity` (`self.PointLight1`) 2500.0)
  (`LightComponent.SetIntensity` (`self.PointLight2`) 2500.0)
  (`LightComponent.SetIntensity` (`self.PointLight3`) 2500.0)
  (`LightComponent.SetIntensity` (`self.PointLight4`) 2500.0)
  (`LightComponent.SetIntensity` (`self.PointLight5`) 2500.0)
  (`LightComponent.SetIntensity` (`self.PointLight6`) 2500.0)
  (`LightComponent.SetIntensity` (`self.PointLight7`) 2500.0))

(event `Light Off`
  (`LightComponent.SetIntensity` (`self.PointLight`) 0.0)
  (`LightComponent.SetIntensity` (`self.PointLight1`) 0.0)
  (`LightComponent.SetIntensity` (`self.PointLight2`) 0.0)
  (`LightComponent.SetIntensity` (`self.PointLight3`) 0.0)
  (`LightComponent.SetIntensity` (`self.PointLight4`) 0.0)
  (`LightComponent.SetIntensity` (`self.PointLight5`) 0.0)
  (`LightComponent.SetIntensity` (`self.PointLight6`) 0.0)
  (`LightComponent.SetIntensity` (`self.PointLight7`) 0.0))

(fn `UserConstructionScript`)