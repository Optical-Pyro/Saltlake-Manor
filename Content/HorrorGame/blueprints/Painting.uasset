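; Painting actor for a horror game that fades part of its material when something enters its trigger box.
; BeginPlay creates a dynamic material instance for the static mesh's material slot 1.
; Box overlap plays a Fade timeline that drives the material's "Fade" scalar parameter, and ending the overlap reverses it.
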(event `self.ReceiveBeginPlay`
  (bind _staticmesh (`self.StaticMesh`))
  (bind _returnvalue (`PrimitiveComponent.CreateDynamicMaterialInstance` _staticmesh 1 (`KismetArrayLibrary.Array_Get` (`MeshComponent.GetMaterials` _staticmesh) 1)))
  (bind _output_get (set `self.TempMat` _returnvalue))
  (`MaterialInstanceDynamic.K2_GetScalarParameterValue` _output_get "Fade"))

(event `self.Box.OnComponentBeginOverlap`
  (params (OverlappedComponent :type "PrimitiveComponent Object Reference") (OtherActor :type "Actor Object Reference") (OtherComp :type "PrimitiveComponent Object Reference") (OtherBodyIndex :type Integer) (bFromSweep :type Boolean) (SweepResult :type "HitResult Structure (by ref)"))
  (bind (_direction _fade) (`Timeline|Fade` :!label _label)
    (:`Update`
      (`/Engine/EditorBlueprintResources/StandardMacros.IsValid` self
        (:`Is Valid`
          (`MaterialInstanceDynamic.SetScalarParameterValue` (`self.TempMat`) "Fade" _fade))))))

(event `self.Box.OnComponentEndOverlap`
  (params (OverlappedComponent :type "PrimitiveComponent Object Reference") (OtherActor :type "Actor Object Reference") (OtherComp :type "PrimitiveComponent Object Reference") (OtherBodyIndex :type Integer))
  (goto _label :!via `Reverse`))

(fn `UserConstructionScript`)