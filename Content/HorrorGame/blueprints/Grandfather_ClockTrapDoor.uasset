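; Grandfather clock trap door actor for a horror game that the player opens by pressing E nearby.
; Overlapping the Trigger enables input, and leaving it disables input.
; Pressing E plays a rumble at the Audio component and moves the Trap along the Open timeline.
; After a fixed delay it plays the rumble again, without the attenuation setting, and reverses the timeline to close the trap.
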(event `self.Trigger.OnComponentBeginOverlap`
  (params (OverlappedComponent :type "PrimitiveComponent Object Reference") (OtherActor :type "Actor Object Reference") (OtherComp :type "PrimitiveComponent Object Reference") (OtherBodyIndex :type Integer) (bFromSweep :type Boolean) (SweepResult :type "HitResult Structure (by ref)"))
  (`self.EnableInput` (`GameplayStatics.GetPlayerController` 0)))

(event `self.Trigger.OnComponentEndOverlap`
  (params (OverlappedComponent :type "PrimitiveComponent Object Reference") (OtherActor :type "Actor Object Reference") (OtherComp :type "PrimitiveComponent Object Reference") (OtherBodyIndex :type Integer))
  (`self.DisableInput` (`GameplayStatics.GetPlayerController` 0)))

(event `Key|E`
  (params (Key :type "Key Structure" :default "AnyKey"))
  (bind _returnvalue (`SceneComponent.K2_GetComponentLocation` (`self.Audio`)))
  (:`Pressed`
    (`|ExecutionSequence`
      (:`then_0`
        (`GameplayStatics.PlaySoundAtLocation` "/Game/HorrorGame/Audio/terrain_rumble1.terrain_rumble1" _returnvalue (struct) 1.0 1.0 0.0 "/Game/HorrorGame/blueprints/GramophoneAttenuation.GramophoneAttenuation")
        (bind (_direction _newtrack_1) (`Timeline|Open` :!label _label)
          (:`Update`
            (`SceneComponent.K2_SetRelativeLocation` (`self.Trap`) _newtrack_1 false false))))
      (:`then_1`
        (`KismetSystemLibrary.Delay` 15.0)
        (`GameplayStatics.PlaySoundAtLocation` "/Game/HorrorGame/Audio/terrain_rumble1.terrain_rumble1" _returnvalue (struct) 1.0 1.0 0.0 "/Game/HorrorGame/blueprints/GramophoneAttenuation.GramophoneAttenuation")
        (goto _label :!via `Reverse`)))))

(fn `UserConstructionScript`)